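; Base puzzle-game character that interacts with nearby objects and can carry boxes.
; An interaction radius tracks the overlapped BPI_Interactable, and IA_Interact begins interaction on trigger and stops it on completion.
; PickupBox and DropBox use the Hands component to grab and release, and Tick holds the grabbed component at a set distance in front of the actor.
; UpdateItemDisplay is an empty stub.
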(event OnComponentBeginOverlap(InteractionRadius)
  (params (OverlappedComponent :type Primitive%20Component%20Object%20Reference) (OtherActor :type Actor%20Object%20Reference) (OtherComp :type Primitive%20Component%20Object%20Reference) (OtherBodyIndex :type Integer) (bFromSweep :type Boolean) (SweepResult :type Hit%20Result%20Structure%20%28by%20ref%29))
  (Utilities|Casting|CastToBPI_Interactable OtherActor)
  (Variables|Default|SetOverlappedInteractable OtherActor))

(event OnComponentEndOverlap(InteractionRadius)
  (params (OverlappedComponent :type Primitive%20Component%20Object%20Reference) (OtherActor :type Actor%20Object%20Reference) (OtherComp :type Primitive%20Component%20Object%20Reference) (OtherBodyIndex :type Integer))
  (if (== OtherActor (Variables|Default|GetOverlappedInteractable))
    (Variables|Default|SetOverlappedInteractable 0)))

(event Input|EnhancedActionEvents|EnhancedInputActionIA_Interact
  (params (ActionValue :type Boolean) (ElapsedSeconds :type Float%20%28double-precision%29) (TriggeredSeconds :type Float%20%28double-precision%29) (InputAction :type Input%20Action%20Object%20Reference :default "/Game/ThirdPerson/Input/Actions/IA_Interact.IA_Interact"))
  (:Triggered
    (bind _overlappedinteractable (Variables|Default|GetOverlappedInteractable)
      (:then
        (bind _asbpi_interactable (Utilities|Casting|CastToBPI_Interactable _overlappedinteractable))
        (Default|BeginInteraction _asbpi_interactable self))
      (:else)))
  (:Completed
    (bind _overlappedinteractable_2 (Variables|Default|GetOverlappedInteractable)
      (:then
        (bind _asbpi_interactable_2 (Utilities|Casting|CastToBPI_Interactable _overlappedinteractable_2))
        (Default|StopInteraction _asbpi_interactable_2 self))
      (:else))))

(event EventTick
  (params (DeltaSeconds :type Float%20%28single-precision%29))
  (if (CallFunction|IsHoldingBox)
    (Physics|Components|PhysicsHandle|SetTargetLocation (Variables|Default|GetHands) (CallFunction|GrabLocation))))

(fn ConstructionScript
  (|CallParentFunction))

(fn PickupBox
  (params (Component :type Primitive%20Component%20Object%20Reference))
  (Class|PhysicsHandleComponent|GrabComponentatLocation (Variables|Default|GetHands) Component "None" (Transformation|GetWorldLocation Component)))

(fn DropBox
  (params (Component :type Primitive%20Component%20Object%20Reference))
  (Physics|Components|PhysicsHandle|ReleaseComponent (Variables|Default|GetHands)))

(fn IsHoldingBox
  (return (Utilities|IsValid (Class|PhysicsHandleComponent|GetGrabbedComponent (Variables|Default|GetHands)))))

(fn GrabLocation
  (return (+ (Transformation|GetActorLocation) (* (Transformation|GetActorForwardVector) (Variables|Default|GetGrabDistance)))))

(fn UpdateItemDisplay)