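; Puzzle game mode child Blueprint that tracks a Score and shows it in an on-screen item display.
; On BeginPlay it creates a WBP_ItemDisplay widget and adds it to the viewport, then pushes Score into it every Tick.
; The UpdateScore event raises Score by a fixed step and tests it against a threshold, but that branch does nothing and NextLevel is unused.
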(event Custom|UpdateScore
  (Variables|Default|SetScore (+ (Variables|Default|GetScore) 2.0))
  (if (>= (Variables|Default|GetScore) 1e+01)
    _))

(event EventBeginPlay
  (bind _returnvalue (UserInterface|CreateWidget "/Game/PuzzleGame/BP_Puzzle/WBP_ItemDisplay.WBP_ItemDisplay_C"))
  (bind _output_get (Variables|Default|SetItemUI _returnvalue))
  (UserInterface|Viewport|AddtoViewport _output_get 0))

(event EventTick
  (params (DeltaSeconds :type Float%20%28single-precision%29))
  (Default|UpdateItemUI (Variables|Default|GetItemUI) (Variables|Default|GetScore)))

(fn ConstructionScript
  (|CallParentFunction))