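; Carryable puzzle cube that a character can pick up and drop through interaction.
; Begin and stop interaction events hand the Cube component to the interacting character's PickupBox and DropBox, so the carry logic lives on the character.
; Overlap by a BP_BaseCharacter reveals a text render, with no logic here to hide it again.
; The construction script tints the cube per instance through a dynamic material's BoxColor parameter.
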(event OnComponentBeginOverlap(OverlapTrigger)
  (params (OverlappedComponent :type Primitive%20Component%20Object%20Reference) (OtherActor :type Actor%20Object%20Reference) (OtherComp :type Primitive%20Component%20Object%20Reference) (OtherBodyIndex :type Integer) (bFromSweep :type Boolean) (SweepResult :type Hit%20Result%20Structure%20%28by%20ref%29))
  (Utilities|Casting|CastToBP_BaseCharacter OtherActor)
  (Rendering|SetVisibility (Variables|Default|GetTextRender) true false))

(event EventBeginInteraction
  (params (InteractingCharacter :type BP%20Base%20Character%20Object%20Reference))
  (Default|PickupBox InteractingCharacter (Variables|Default|GetCube)))

(event EventStopInteraction
  (params (InteractingCharacter :type BP%20Base%20Character%20Object%20Reference))
  (Default|DropBox InteractingCharacter (Variables|Default|GetCube)))

(fn ConstructionScript
  (bind _returnvalue (Rendering|Material|CreateDynamicMaterialInstance (Variables|Default|GetCube) 0 0 "None" :!class /Script/Engine.PrimitiveComponent))
  (Rendering|Material|SetVectorParameterValue _returnvalue "BoxColor" (Variables|Default|GetBoxColor) :!class /Script/Engine.MaterialInstanceDynamic))

(fn CreateMaterial)