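; BP_PaintBucket is a puzzle actor that recolors carryable cubes on contact.
; Its construction script creates a dynamic material on the bucket mesh and tints it with the PaintColor variable.
; When a BP_CarryCube begins overlapping the capsule, PaintColorWithBucket applies that color to the cube's material and stores it in the cube's BoxColor variable.
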(event OnComponentBeginOverlap(Capsule)
  (params (OverlappedComponent :type Primitive%20Component%20Object%20Reference) (OtherActor :type Actor%20Object%20Reference) (OtherComp :type Primitive%20Component%20Object%20Reference) (OtherBodyIndex :type Integer) (bFromSweep :type Boolean) (SweepResult :type Hit%20Result%20Structure%20%28by%20ref%29))
  (CallFunction|PaintColorwithBucket OtherActor))

(fn ConstructionScript
  (Rendering|Material|CreateDynamicMaterialInstance (Variables|Default|GetPaintBucketMesh) 0 0 "None" :!class /Script/Engine.PrimitiveComponent)
  (Rendering|Material|SetVectorParameterValueonMaterials (Variables|Default|GetPaintBucketMesh) "PaintColor" (Math|Conversions|ToVector(LinearColor) (Variables|Default|GetPaintColor))))

(fn PaintColorwithBucket
  (params (Object :type Object%20Object%20Reference))
  (bind _asbp_carry_cube (Utilities|Casting|CastToBP_CarryCube Object))
  (bind _output_get (Variables|Default|SetAs%20BP%20Carry%20Cube _asbp_carry_cube))
  (Rendering|Material|SetVectorParameterValueonMaterials (Variables|/Game/PuzzleGame/BP_Puzzle/BP_CarryCube.BP_CarryCube_C|GetCube _output_get) "BoxColor" (Math|Conversions|ToVector(LinearColor) (Variables|Default|GetPaintColor)))
  (Variables|/Game/PuzzleGame/BP_Puzzle/BP_CarryCube.BP_CarryCube_C|SetBoxColor (Variables|Default|GetAs%20BP%20Carry%20Cube) (Variables|Default|GetPaintColor)))